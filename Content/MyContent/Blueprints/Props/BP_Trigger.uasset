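; BP_Trigger is a one-shot button prop that opens a linked door when something overlaps its collider.
; On BeginPlay it creates a dynamic material instance for the Button mesh.
; The first overlap destroys the collider, turns the button bright green and plays a timeline that drives the actor's Z position.
; When the timeline finishes, it plays a success sound and calls OpenDoor on DoorToTrigger.
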(event OnComponentBeginOverlap(Collider)
  (params (OverlappedComponent :type Primitive%20Component%20Object%20Reference) (OtherActor :type Actor%20Object%20Reference) (OtherComp :type Primitive%20Component%20Object%20Reference) (OtherBodyIndex :type Integer) (bFromSweep :type Boolean) (SweepResult :type Hit%20Result%20Structure%20%28by%20ref%29))
  (bind _returnvalue (Transformation|GetActorLocation))
  (Components|DestroyComponent (Variables|Default|GetCollider))
  (Rendering|Material|SetVectorParameterValue (Variables|Default|GetDynamicMaterialInstance) "Color" "(R=0.000000,G=3.000000,B=0.000000,A=1.000000)" :!class /Script/Engine.MaterialInstanceDynamic)
  (bind _newz (Timeline|TriggerTimeline PlayFromStart)
    (:Update
      (Transformation|SetActorLocation (Math|Vector|MakeVector (.x _returnvalue) (.y _returnvalue) _newz) false false))
    (:Finished
      (Audio|PlaySound2D "/Engine/EditorSounds/Notifications/CompileSuccess.CompileSuccess" 1.0 1.0 0.0 0 0)
      (Default|OpenDoor (Variables|Setup|GetDoorToTrigger)))))

(event EventBeginPlay
  (bind _returnvalue (Rendering|Material|CreateDynamicMaterialInstance (Variables|Default|GetButton) 0 0 "None" :!class /Script/Engine.PrimitiveComponent))
  (Variables|Default|SetDynamicMaterialInstance _returnvalue))

(fn ConstructionScript)